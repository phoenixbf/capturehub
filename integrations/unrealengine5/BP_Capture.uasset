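; BP_Capture records an actor's eye viewpoint over time and targets a hub's HTTP session API with the data.
; On BeginPlay it starts a looping Capture timer, finds the actor by class, and POSTs field names and actor name to obtain a session id.
; Once a session exists, Trace appends timestamped location and rotation as CSV rows.
; When the count exceeds the chunk size, it creates a PUT request with the chunk, then resets the buffer.
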(event Custom|Capture
  (CallFunction|Trace))

(event EventBeginPlay
  (Utilities|Time|SetTimerbyFunctionName 0 "Capture" (Variables|Default|GetInterval) true)
  (bind _returnvalue (Actor|GetActorOfClass (Variables|Default|Getactorclass)))
  (if (Utilities|IsValid _returnvalue)
    (Variables|Default|Setactor _returnvalue)
    (bind _result_body (|HttpRequest :Url (Utilities|String|Append (Variables|Default|Gethubaddress) "/api/session") :Verb "Post" :Body (Utilities|String|Append "{\"fields\":[" (Variables|Default|Getattributes) "],\"actor\":\"" (Variables|Default|Getactorname) "\"}"))
      (:On%20Success
        (bind (_outvalue _returnvalue_2) (|GetJsonField _result_body "id"))
        (if _returnvalue_2
          (bind _output_get (Variables|Default|Setsessionid _outvalue))
          (Variables|Default|SetbSession _returnvalue_2)
          (Development|PrintString _output_get)))
      (:On%20Error
        (Development|PrintString "FAIL" true true "(R=1.000000,G=0.000000,B=0.000000,A=1.000000)")))))

(fn ConstructionScript)

(fn Trace
  (bind _actor (Variables|Default|Getactor))
  (bind _counter (Variables|Default|Getcounter))
  (bind (_outlocation _outrotation) (Actor|GetActorEyesViewPoint _actor))
  (if (Variables|Default|GetbSession)
    (Variables|Default|Setdatachunk (Utilities|String|Append (Variables|Default|Getdatachunk) (Utilities|String|Append (Utilities|String|ToString(Float) (Utilities|Time|GetTimeSeconds)) "," (Utilities|String|ToString(Float) (.x _outlocation)) "," (Utilities|String|ToString(Float) (.y _outlocation)) "," (Utilities|String|ToString(Float) (.z _outlocation)) "," (Utilities|String|ToString(Float) (.roll _outrotation)) "," (Utilities|String|ToString(Float) (.pitch _outrotation)) "," (Utilities|String|ToString(Float) (.yaw _outrotation)) "\\n")))
    (Math|Integer|IncrementInt _counter
      (:%20%20
        (if (> _counter (Variables|Default|Getchunksize))
          (Development|PrintString (Utilities|String|Append "{\"id\":\"" (Variables|Default|Getsessionid) "\",\"data\":\"" (Variables|Default|Getdatachunk) "\"}"))
          (Class|HttpRequestProxyObject|CreateHttpRequestProxyObject :InUrl (Utilities|String|Append (Variables|Default|Gethubaddress) "/api/session") :InVerb "PUT" :InBody (Utilities|String|Append "{\"id\":\"" (Variables|Default|Getsessionid) "\",\"data\":\"" (Variables|Default|Getdatachunk) "\"}"))
          (CallFunction|ResetDataChunk))))))

(fn ResetDataChunk
  (Variables|Default|Setdatachunk "")
  (Variables|Default|Setcounter 0))